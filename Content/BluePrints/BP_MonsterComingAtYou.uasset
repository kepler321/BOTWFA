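; BP_MonsterComingAtYou is a scripted monster scare actor, driven by three overlap triggers.
; The monster starts hidden; the first trigger reveals it, plays a walk sound and slides it to a goal component with MoveComponentTo.
; The second resets its rotation in place, and both triggers destroy themselves after use.
; The third plays a jumpscare sound, snaps the monster to the relative origin and destroys the actor.
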(event `self.ReceiveBeginPlay`
  (`SceneComponent.SetVisibility` (`self.Monster`) false false))

(event `self.FirstTrigger.OnComponentBeginOverlap`
  (params (OverlappedComponent :type "PrimitiveComponent Object Reference") (OtherActor :type "Actor Object Reference") (OtherComp :type "PrimitiveComponent Object Reference") (OtherBodyIndex :type Integer) (bFromSweep :type Boolean) (SweepResult :type "HitResult Structure (by ref)"))
  (bind _monster (`self.Monster`))
  (`GameplayStatics.PlaySound2D` "/Game/Sounds/SFX_MonsterWalkBlueGem_Cue.SFX_MonsterWalkBlueGem_Cue" 1.0 1.0 0.0 null null)
  (`SceneComponent.SetVisibility` _monster true false)
  (`KismetSystemLibrary.MoveComponentTo` _monster (`SceneComponent.RelativeLocation` (`self.GoalFirstTrigger`)) (struct :`Yaw` -90.0) false false 1.5)
  (`ActorComponent.K2_DestroyComponent` (`self.FirstTrigger`)))

(event `self.SecondTrigger.OnComponentBeginOverlap`
  (params (OverlappedComponent :type "PrimitiveComponent Object Reference") (OtherActor :type "Actor Object Reference") (OtherComp :type "PrimitiveComponent Object Reference") (OtherBodyIndex :type Integer) (bFromSweep :type Boolean) (SweepResult :type "HitResult Structure (by ref)"))
  (`KismetSystemLibrary.MoveComponentTo` (`self.Monster`) (`SceneComponent.RelativeLocation` (`self.Monster`)) (struct) false false 1.0)
  (`ActorComponent.K2_DestroyComponent` (`self.SecondTrigger`)))

(event `self.ThirdTrigger.OnComponentBeginOverlap`
  (params (OverlappedComponent :type "PrimitiveComponent Object Reference") (OtherActor :type "Actor Object Reference") (OtherComp :type "PrimitiveComponent Object Reference") (OtherBodyIndex :type Integer) (bFromSweep :type Boolean) (SweepResult :type "HitResult Structure (by ref)"))
  (`GameplayStatics.PlaySound2D` "/Game/Sounds/SFX_BlueGemMonsterJS_Cue.SFX_BlueGemMonsterJS_Cue" 1.0 1.0 0.0 null null)
  (`KismetSystemLibrary.MoveComponentTo` (`self.Monster`) (0.0 0.0 0.0) (struct) false false 0.3)
  (`self.K2_DestroyActor`))

(fn `UserConstructionScript`)